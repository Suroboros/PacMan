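; Pac-Man enemy that chases the player and restarts the game on contact.
; It starts idle and begins hunting after a short delay, with a state-changed event driving movement updates.
; AI MoveToActor pursues the player pawn in every state except Idle, which stops movement.
; A mesh hit on Pac-Man teleports the player far away, idles the enemy, then opens Level_01 after a delay.
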(event OnComponentHit(StaticMesh)
  (params (HitComponent :type Primitive%20Component%20Object%20Reference) (OtherActor :type Actor%20Object%20Reference) (OtherComp :type Primitive%20Component%20Object%20Reference) (NormalImpulse :type Vector :default "0, 0, 0") (Hit :type Hit%20Result%20Structure%20%28by%20ref%29))
  (bind _aspac_man_bp (Utilities|Casting|CastToPacMan_BP OtherActor))
  (Transformation|SetActorLocation _aspac_man_bp "10000.000000,10000.000000,10000.000000" false false)
  (Class|EnemyPawn|Idle)
  (Utilities|FlowControl|Delay 2.0)
  (Game|OpenLevel(byName) "Level_01"))

(event Custom|Setup%20State%20Changed%20Event
  (EventDispatchers|BindEventtoStateChangedEvent (delegate Custom|Event%20State%20Changed)))

(event Custom|Event%20State%20Changed
  (params (New%20State :type EEnemyState%20Enum :default "Default"))
  (CallFunction|UpdateMovement))

(event EventBeginPlay
  (CallFunction|SetupStateChangedEvent)
  (Class|EnemyPawn|Idle)
  (Utilities|FlowControl|Delay 1.5)
  (Class|EnemyPawn|Hunt))

(event Collision|EventActorBeginOverlap
  (params (OtherActor :type Actor%20Object%20Reference)))

(event EventTick
  (params (DeltaSeconds :type Float%20%28single-precision%29)))

(fn ConstructionScript)

(fn UpdateMovement
  (LocalVariables|SetAIController (AI|GetAIController (Pawn|GetController)))
  (switch Utilities|FlowControl|Switch|SwitchonEEnemyState (Variables|Default|GetState)
    (:Default
      (AI|Navigation|MovetoActor (LocalVariables|GetAIController) (Game|Player|GetPlayerPawn 0) 0.0 false true true 0))
    (:Idle
      (AI|Navigation|StopMovement (LocalVariables|GetAIController)))))
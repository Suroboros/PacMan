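; Pac-Man pawn Blueprint that handles the start-of-play unfreeze and a timed movement power-up.
; BeginPlay waits two seconds, then calls SetFrozen(false).
; EnablePowerUpMovement applies power-up max speed and acceleration to the FloatingPawnMovement component, then fires the PowerUpEffect event.
; That event waits for the power-up duration, then calls EnableNormalMovement to restore the normal movement values.
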(event Custom|Power%20Up%20Effect
  (Utilities|FlowControl|Delay (Variables|Default|GetPower%20Up%20Duration))
  (CallFunction|EnableNormalMovement))

(event EventBeginPlay
  (Utilities|FlowControl|Delay 2.0)
  (Class|PacManPawn|SetFrozen false))

(event Collision|EventActorBeginOverlap
  (params (OtherActor :type Actor%20Object%20Reference)))

(event EventTick
  (params (DeltaSeconds :type Float%20%28single-precision%29)))

(fn ConstructionScript)

(fn EnableNormalMovement
  (bind _floatingpawnmovement (Variables|Default|GetFloatingPawnMovement))
  (Utilities|FlowControl|Sequence
    (:then_0
      (Variables|/Script/Engine.FloatingPawnMovement|SetMaxSpeed _floatingpawnmovement (Variables|Default|GetNormal%20Speed)))
    (:then_1
      (Variables|/Script/Engine.FloatingPawnMovement|SetAcceleration _floatingpawnmovement (Variables|Default|GetNarmal%20Acceleration)))))

(fn EnablePowerUpMovement
  (bind _floatingpawnmovement (Variables|Default|GetFloatingPawnMovement))
  (Utilities|FlowControl|Sequence
    (:then_0
      (Variables|/Script/Engine.FloatingPawnMovement|SetMaxSpeed _floatingpawnmovement (Variables|Default|GetPower%20Up%20Speed)))
    (:then_1
      (Variables|/Script/Engine.FloatingPawnMovement|SetAcceleration _floatingpawnmovement (Variables|Default|GetPower%20Up%20Acceleration)))
    (:then_2
      (CallFunction|PowerUpEffect))))